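; Physics-driven boat that chases the collision sphere of the first Boat_Spline actor in the level, starting four seconds after BeginPlay.
; MoveTo re-runs itself through a tiny Delay, easing rotation toward the sphere while applying force, or setting velocity to Speed when above it.
; Tick holds the jib pivot at a fixed world yaw, and a missing sphere prints a warning.
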(event Custom|MoveTo
  (bind _returnvalue (Transformation|GetActorLocation))
  (bind _speed (Variables|Default|GetSpeed))
  (bind _sphere_collision (Variables|Default|GetSphere%20Collision))
  (bind _returnvalue_2 (Transformation|GetWorldLocation _sphere_collision))
  (bind _returnvalue_3 (Math|Vector|GetUnitDirection(Vector) _returnvalue _returnvalue_2))
  (bind (_x _y) (Math|Vector|BreakVector _returnvalue_3))
  (bind _returnvalue_4 (* _returnvalue_3 _speed))
  (Utilities|IsValid _sphere_collision
    (:Is%20Valid
      (Transformation|SetActorRotation (Math|Interpolation|RInterpTo (Transformation|GetWorldRotation (Variables|Default|GetBoatCollision)) (Math|Rotator|MakeRotator _x _y (- (.yaw (Math|Conversions|RotationFromXVector _returnvalue_3)) 9e+01)) (Utilities|Time|GetWorldDeltaSeconds) 1.0))
      (bind _returnvalue_5 (Physics|GetPhysicsLinearVelocity (Variables|Default|GetBoatCollision) "None"))
      (if (> (Math|Vector|VectorLength _returnvalue_5) (Variables|Default|GetSpeed))
        (Physics|SetPhysicsLinearVelocity (Variables|Default|GetBoatCollision) _returnvalue_4 false "None")
        (Utilities|FlowControl|Delay 0.001)
        (CallFunction|Moveto)
        (else
          (Physics|AddForce (Variables|Default|GetBoatCollision) _returnvalue_4 "None" true)
          (Utilities|FlowControl|Delay 0.001)
          (CallFunction|Moveto))))
    (:Is%20Not%20Valid
      (Development|PrintString "Add a  BoatSpline to scene!"))))

(event EventBeginPlay
  ;[1 1 1] Begin
  (Utilities|FlowControl|Delay 4.0)
  (bind _outactors (Actor|GetAllActorsOfClass "/Game/TimeWalk/Boat_Spline.Boat_Spline_C"))
  (Variables|Default|SetSphere%20Collision (Variables|/Game/TimeWalk/Boat_Spline.Boat_Spline_C|GetSphereCollision (Utilities|Array|Get(acopy) _outactors)))
  (CallFunction|Moveto))

(event EventTick
  (params (DeltaSeconds :type Float%20%28single-precision%29))
  (bind __jib_pivot (Variables|Default|Get_Jib_pivot))
  (bind _returnvalue (Transformation|GetWorldRotation __jib_pivot))
  (bind (_roll _pitch) (Math|Rotator|BreakRotator _returnvalue))
  (Transformation|SetWorldRotation __jib_pivot (Math|Rotator|MakeRotator _roll _pitch 9e+01) false false))

(fn ConstructionScript)

(fn NewFunction
  (params (self2 :type Boat%20Spline%20Object%20Reference))
  (Class|PrimitiveComponent|BoxOverlapComponent :self (Variables|/Game/TimeWalk/Boat_Spline.Boat_Spline_C|GetSphereCollision self2)))